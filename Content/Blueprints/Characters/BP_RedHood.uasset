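; BP_RedHood is the player character for Red Hood, with side-scrolling style movement along the world X axis and jumping.
; On BeginPlay it adds the IMC_RedHood Enhanced Input mapping context to its player controller.
; The move action applies rounded input as movement, then snaps controller yaw to 0 or 180 from the sign of X acceleration to face the travel direction.
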(event Input|EnhancedActionEvents|EnhancedInputActionIA_Move
  (params (ActionValue :type Float%20%28double-precision%29) (ElapsedSeconds :type Float%20%28double-precision%29) (TriggeredSeconds :type Float%20%28double-precision%29) (InputAction :type Input%20Action%20Object%20Reference :default "/Game/Input/IA_Move.IA_Move"))
  (Pawn|Input|AddMovementInput "1.000000,0.000000,0.000000" (Math|Conversions|ToFloat(Integer) (Math|Float|Round ActionValue)) false)
  (CallFunction|RotateController))

(event Input|EnhancedActionEvents|EnhancedInputActionIA_Jump
  (params (ActionValue :type Boolean) (ElapsedSeconds :type Float%20%28double-precision%29) (TriggeredSeconds :type Float%20%28double-precision%29) (InputAction :type Input%20Action%20Object%20Reference :default "/Game/Input/IA_Jump.IA_Jump"))
  (Character|Jump))

(event EventBeginPlay
  (CallFunction|AddPlayerMappingContext))

(fn ConstructionScript)

(fn AddPlayerMappingContext
  (bind _asplayer_controller (Utilities|Casting|CastToPlayerController (Pawn|GetController)))
  (Input|AddMappingContext (PlayerController|LocalPlayerSubsystems|GetEnhancedInputLocalPlayerSubsystem _asplayer_controller) "/Game/Input/IMC_RedHood.IMC_RedHood" 0 "(bIgnoreAllPressedKeysUntilRelease=True,bForceImmediately=False,bNotifyUserSettings=False)"))

(fn RotateController
  (Math|Float|CompareFloat (.x (Pawn|Components|CharacterMovement|GetCurrentAcceleration (Variables|Character|GetCharacterMovement))) 0.0
    (:>
      (LocalVariables|SetrotationAngle 0.0))
    (:<
      (LocalVariables|SetrotationAngle 1.8e+02)))
  (Pawn|SetControlRotation (Pawn|GetController) (Math|Rotator|MakeRotator 0.0 0.0 (LocalVariables|GetrotationAngle))))